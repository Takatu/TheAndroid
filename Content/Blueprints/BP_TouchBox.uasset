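; BP_TouchBox is a skeletal-mesh box that changes color when its OnTouch event fires.
; The construction script creates and stores a dynamic material instance, starts the non-looping morph animation, then writes animation data with a random saved position, apparently to vary each box's shape.
; OnTouch sets the BaseColor_A and BaseColor_B vector parameters on that material to a fixed green and blue.
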(event `OnTouch`
  (bind _material (`self.Material`))
  (`MaterialInstanceDynamic.SetVectorParameterValue` _material "BaseColor_A" (struct :`R` 0.0478 :`G` 0.32 :`A` 1.0))
  (`MaterialInstanceDynamic.SetVectorParameterValue` _material "BaseColor_B" (struct :`R` 0.033167 :`B` 0.69 :`A` 1.0)))

(fn `UserConstructionScript`
  (bind _skeletalmesh1 (`self.SkeletalMesh1`))
  (bind _returnvalue (`PrimitiveComponent.CreateDynamicMaterialInstance` (`self.SkeletalMesh1`) 0 null))
  (set `self.Material` _returnvalue)
  (`SkeletalMeshComponent.PlayAnimation` _skeletalmesh1 "/Game/ExampleContent/Morph_Targets/Morph_1/SK_Box_Morph_1_Anim.SK_Box_Morph_1_Anim" false)
  (set `SkeletalMeshComponent.AnimationData` (make `SkeletalMeshComponent.SingleAnimationPlayData` "/Game/ExampleContent/Morph_Targets/Morph_1/SK_Box_Morph_1_Anim.SK_Box_Morph_1_Anim" true true (`KismetMathLibrary.RandomFloat`)) _skeletalmesh1))